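; Traffic light actor that endlessly cycles green, yellow and red by setting scalar parameters on a dynamic material instance.
; The construction script creates that instance on the TrafficLight1Lane component, and BeginPlay runs a looping chain of Delays.
; TrafficLightOffeset picks whether the cycle starts on green or red, putting lights in opposite phases.
; Red lasts the full TrafficLightLength, while green and yellow each last half.
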(event `self.ReceiveBeginPlay`
  (bind _trafficlight_dmi (`self.TrafficLight_DMI`))
  (bind _trafficlight_length (`self.TrafficLight_Length`))
  (bind _returnvalue (- _trafficlight_length (/ _trafficlight_length 2.0)))
  (if (`self.TrafficLight_Offeset`)
    (`MaterialInstanceDynamic.SetScalarParameterValue` _trafficlight_dmi "GreenLight" 1.0 :!label _label)
    (`MaterialInstanceDynamic.SetScalarParameterValue` _trafficlight_dmi "RedLight" 0.0)
    (`KismetSystemLibrary.Delay` _returnvalue)
    (`MaterialInstanceDynamic.SetScalarParameterValue` _trafficlight_dmi "YellowLight" 1.0)
    (`MaterialInstanceDynamic.SetScalarParameterValue` _trafficlight_dmi "GreenLight" 0.0)
    (`KismetSystemLibrary.Delay` _returnvalue)
    (`MaterialInstanceDynamic.SetScalarParameterValue` _trafficlight_dmi "RedLight" 1.0)
    (`MaterialInstanceDynamic.SetScalarParameterValue` _trafficlight_dmi "YellowLight" 0.0)
    (`KismetSystemLibrary.Delay` (`self.TrafficLight_Length`))
    (goto _label)
    (else
      (`MaterialInstanceDynamic.SetScalarParameterValue` _trafficlight_dmi "RedLight" 1.0 :!label _label_2)
      (`MaterialInstanceDynamic.SetScalarParameterValue` _trafficlight_dmi "GreenLight" 0.0)
      (`MaterialInstanceDynamic.SetScalarParameterValue` _trafficlight_dmi "YellowLight" 0.0)
      (`KismetSystemLibrary.Delay` _trafficlight_length)
      (`MaterialInstanceDynamic.SetScalarParameterValue` _trafficlight_dmi "RedLight" 0.0)
      (`MaterialInstanceDynamic.SetScalarParameterValue` _trafficlight_dmi "GreenLight" 1.0)
      (`KismetSystemLibrary.Delay` _returnvalue)
      (`MaterialInstanceDynamic.SetScalarParameterValue` _trafficlight_dmi "YellowLight" 1.0)
      (`MaterialInstanceDynamic.SetScalarParameterValue` _trafficlight_dmi "GreenLight" 0.0)
      (`KismetSystemLibrary.Delay` _returnvalue)
      (goto _label_2))))

(event `self.ReceiveActorBeginOverlap`
  (params (OtherActor :type "Actor Object Reference")))

(event `self.ReceiveTick`
  (params (DeltaSeconds :type "Float (single-precision)")))

(fn `UserConstructionScript`
  (bind _returnvalue (`PrimitiveComponent.CreateDynamicMaterialInstance` (`self.TrafficLight_1Lane`) 0 "/Game/IndustrialCity/Materials/-TrafficLight.-TrafficLight"))
  (set `self.TrafficLight_DMI` _returnvalue))
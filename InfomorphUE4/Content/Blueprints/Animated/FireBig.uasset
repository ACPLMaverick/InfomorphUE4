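; FireBig is a fire hazard actor that damages characters standing within its sphere.
; On BeginPlay it plays a fire sound cue at its location.
; Each Tick it polls the sphere for overlapping BaseCharacter_BP actors and calls damage on their HitComp, scaling DamagePerSecond by delta time.
; Each victim's own controller is passed as the instigator, with the fire as damage causer.
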(event `self.ReceiveBeginPlay`
  (`GameplayStatics.PlaySoundAtLocation` "/Game/Audio/SFX/Cues/Fire01_Cue.Fire01_Cue" (`self.K2_GetActorLocation`)))

(event `self.ReceiveTick`
  (params (DeltaSeconds :type "Float (single-precision)"))
  (for _array_element (`PrimitiveComponent.GetOverlappingActors` (`self.Sphere`) "/Game/Blueprints/Characters/BaseCharacter_BP.BaseCharacter_BP_C")
    (bind _asbase_character_bp (cast `/Game/Blueprints/Characters/BaseCharacter_BP` _array_element))
    (`/Game/Blueprints/CharacterUtility/HitComp.EventDamage` (`/Game/Blueprints/Characters/BaseCharacter_BP.HitComp` _asbase_character_bp) _asbase_character_bp (* (`GameplayStatics.GetWorldDeltaSeconds`) (`self.DamagePerSecond`)) null (`Pawn.GetController` _asbase_character_bp) self)))

(fn `UserConstructionScript`)
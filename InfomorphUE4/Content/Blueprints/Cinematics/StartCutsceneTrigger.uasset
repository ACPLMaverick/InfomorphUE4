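; Cutscene trigger for the game's start cutscene, in which a possession actor takes over a Grunt.
; On BeginPlay it registers with the Infomorph game mode as "StartCutscene" and hides both actors.
; Cutscene events show the Grunt, enable player input, then after a delay send the possession actor above the Grunt to possess it and vanish.
; On end it destroys both actors; it also supplies a fixed playback end time.
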(event `self.ReceiveBeginPlay`
  (`parent.ReceiveBeginPlay`)
  (bind _asinfomorph_game_mode_bp (cast `/Game/Blueprints/InfomorphGameMode_BP` (`GameplayStatics.GetGameMode`)))
  (`BlueprintMapLibrary.Map_Add` (`/Game/Blueprints/InfomorphGameMode_BP.CutsceneControllers` _asinfomorph_game_mode_bp) "StartCutscene" self)
  (`self.SetActorHiddenInGame` (`self.PossessionActor`) true)
  (`self.SetActorHiddenInGame` (`self.GruntActor`) true))

(event `self.EventCutsceneBegin`
  (`parent.EventCutsceneBegin`)
  (`/Game/CustomContent/Cinematics/PossessedGruntPseudoActor.EventAppear` (`self.GruntActor`))
  (`self.EnableInput` (`GameplayStatics.GetPlayerController` 0)))

(event `EventCutsceneAppear`
  (params (DelayToPossession :type "Float (double-precision)"))
  (bind _possessionactor (`self.PossessionActor`))
  (`/Game/CustomContent/Cinematics/PossessionPseudoActor.EventAppear` _possessionactor)
  (`KismetSystemLibrary.Delay` DelayToPossession)
  (`/Game/CustomContent/Cinematics/PossessionPseudoActor.EventGotoLocation` _possessionactor (+ (`self.K2_GetActorLocation` (`self.GruntActor`)) (0.0 0.0 160.0)))
  (`KismetSystemLibrary.Delay` 0.5)
  (`/Game/CustomContent/Cinematics/PossessedGruntPseudoActor.EventPossess` (`self.GruntActor`))
  (`/Game/CustomContent/Cinematics/PossessionPseudoActor.EventDisappear` (`self.PossessionActor`)))

(event `self.EventCutsceneEnd`
  (bind _gruntactor (`self.GruntActor`))
  (bind _possessionactor (`self.PossessionActor`))
  (`parent.EventCutsceneEnd`)
  (`/Game/CustomContent/Cinematics/PossessedGruntPseudoActor.EventDisappear` (`self.GruntActor`))
  (`|ExecutionSequence`
    (:`then_0`
      (if (`KismetSystemLibrary.IsValid` _possessionactor)
        (`self.K2_DestroyActor` _possessionactor)))
    (:`then_1`
      (if (`KismetSystemLibrary.IsValid` _gruntactor)
        (`self.K2_DestroyActor` _gruntactor)))))

(fn `GetPlaybackEndTime`
  (returns (EndTime :type "Float (double-precision)"))
  (return 37.333336))

(fn `UserConstructionScript`
  (`parent.UserConstructionScript`))
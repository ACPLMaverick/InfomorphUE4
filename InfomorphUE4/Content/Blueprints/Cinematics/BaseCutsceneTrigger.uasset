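; Base cutscene trigger actor that plays a Level Sequence on overlap or optionally at BeginPlay, destroying itself when playback stops.
; Tick times a skip-hint widget's appearance and disappearance during playback.
; Enter, E or gamepad bottom button jumps playback to GetPlaybackEndTime, hardcoded here to 1.0.
; Cutscene begin/end events, not called within this Blueprint, toggle the Infomorph player controller and input, with end also removing the widget.
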(event `self.ReceiveBeginPlay`
  (`|ExecutionSequence`
    (:`then_0`
      (if (`self.bStartOnBeginPlay`)
        (bind _pl (`self.IsPlaying`))
        (if (not _pl)
          (`self.PlaySequence`))))
    (:`then_1`
      (bind _returnvalue (`|CreateWidget` "/Game/CustomContent/Blueprints/GUI/SkipCutscene.SkipCutscene_C" (`GameplayStatics.GetPlayerController` 0)))
      (set `self.WidgetSkip` _returnvalue))))

(event `Key|Gamepad_FaceButton_Bottom`
  (params (Key :type "Key Structure" :default "AnyKey"))
  (:`Pressed`
    (bind _pl (`self.IsPlaying` :!label _label))
    (if _pl
      (bind _endtime (`self.GetPlaybackEndTime`))
      (`MovieSceneSequencePlayer.SetPlaybackPosition` (`self.Player`) _endtime))))

(event `Key|Enter` :paused true
  (params (Key :type "Key Structure" :default "AnyKey"))
  (:`Pressed`
    (goto _label)))

(event `Key|E`
  (params (Key :type "Key Structure" :default "AnyKey"))
  (:`Pressed`
    (goto _label)))

(event `self.ReceiveTick`
  (params (DeltaSeconds :type "Float (single-precision)"))
  (bind _timer (`self.Timer`))
  (bind _pl (`self.IsPlaying`))
  (if _pl
    (set `self.Timer` (+ (`self.Timer`) DeltaSeconds))
    (`|ExecutionSequence`
      (:`then_0`
        (if (and (> _timer (`self.SkipHelperAppearTime`)) (not (`self.bSkipInfoVisible`)) (<= _timer (`self.SkipHelperDisappearTime`)))
          (`self.EventSkipInfoAppear`)))
      (:`then_1`
        (if (and (> (`self.Timer`) (`self.SkipHelperDisappearTime`)) (`self.bSkipInfoVisible`))
          (`self.EventSkipInfoDisappear`))))))

(event `self.ReceiveActorBeginOverlap`
  (params (OtherActor :type "Actor Object Reference"))
  (bind _pl (`self.IsPlaying`))
  (if (not _pl)
    (`self.PlaySequence`)))

(event `PlaySequence`
  (bind _sequence (`self.Sequence`))
  (`PrimitiveComponent.SetCollisionEnabled` (`self.Trigger`) "NoCollision")
  (`/Engine/EditorBlueprintResources/StandardMacros.IsValid` _sequence
    (:`Is Valid`
      (bind _returnvalue (`LevelSequencePlayer.CreateLevelSequencePlayer` self _sequence))
      (bind _output_get (set `self.Player` _returnvalue))
      (`MovieSceneSequencePlayer.Play` _returnvalue)
      (add `MovieSceneSequencePlayer.OnStop` _output_get (delegate `OnSequenceStop`)))))

(event `OnSequenceStop`
  (`self.K2_DestroyActor`))

(event `EventCutsceneBegin`
  (bind _asinfomorph_player_controller_bp (cast `/Game/Blueprints/Controllers/InfomorphPlayerController_BP` (`GameplayStatics.GetPlayerController` 0)))
  (`/Game/Blueprints/Controllers/InfomorphPlayerController_BP.Disable` _asinfomorph_player_controller_bp)
  (`self.EnableInput` (`GameplayStatics.GetPlayerController` 0) null))

(event `EventCutsceneEnd`
  (`self.DisableInput` (`GameplayStatics.GetPlayerController` 0))
  (bind _asinfomorph_player_controller_bp (cast `/Game/Blueprints/Controllers/InfomorphPlayerController_BP` (`GameplayStatics.GetPlayerController` 0)))
  (`/Game/Blueprints/Controllers/InfomorphPlayerController_BP.Enable` _asinfomorph_player_controller_bp)
  (`Widget.RemoveFromParent` (`self.WidgetSkip`)))

(event `EventSkipInfoAppear`
  (bind _widgetskip (`self.WidgetSkip`))
  (`/Engine/EditorBlueprintResources/StandardMacros.IsValid` _widgetskip
    (:`Is Valid`
      (set `self.bSkipInfoVisible` true)
      (`UserWidget.AddToViewport` _widgetskip 0)
      (`/Game/CustomContent/Blueprints/GUI/SkipCutscene.WidgetAppear` _widgetskip))))

(event `EventSkipInfoDisappear`
  (bind _widgetskip (`self.WidgetSkip`))
  (`/Engine/EditorBlueprintResources/StandardMacros.IsValid` _widgetskip
    (:`Is Valid`
      (set `self.bSkipInfoVisible` false)
      (`/Game/CustomContent/Blueprints/GUI/SkipCutscene.WidgetDisappear` _widgetskip))))

(fn `GetPlaybackEndTime`
  (returns (EndTime :type "Float (double-precision)"))
  (return 1.0))

(fn `IsPlaying`
  (returns (Pl :type Boolean))
  (bind _player (`self.Player`))
  (if (`KismetSystemLibrary.IsValid` _player)
    (if (`MovieSceneSequencePlayer.IsPlaying` _player)
      (return true)
      (else
        _)))
  (return false))

(fn `UserConstructionScript`)
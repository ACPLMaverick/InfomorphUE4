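; Player controller Blueprint that toggles the player's on-screen presence and provides debug hotkeys.
; Enable and Disable make the child-actor HUD controller appear or disappear, then show or hide the controlled BaseCharacter_BP and its weapon.
; Their shield branches check the shield but target the character or controller instead, and input toggling is disconnected.
; F1–F4 toggle god mode, restart the level, open the splash map and teleport the pawn along camera forward.
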(event `Enable`
  (bind _asplayer_hudcontroller (cast `/Game/Blueprints/CharacterUtility/PlayerHUDController` (`ChildActorComponent.ChildActor` (`self.HUDController`))))
  (`/Game/Blueprints/CharacterUtility/PlayerHUDController.Appear` _asplayer_hudcontroller)
  (bind _asbase_character_bp (cast `/Game/Blueprints/Characters/BaseCharacter_BP` (`self.K2_GetPawn`)))
  (`self.SetActorHiddenInGame` _asbase_character_bp false)
  (`|ExecutionSequence`
    (:`then_0`
      (bind _returnvalue (`InfomorphUE4Character.GetCurrentWeapon` _asbase_character_bp))
      (`/Engine/EditorBlueprintResources/StandardMacros.IsValid` _returnvalue
        (:`Is Valid`
          (`self.SetActorHiddenInGame` _returnvalue false))))
    (:`then_1`
      (bind _returnvalue_2 (`InfomorphUE4Character.GetCurrentShield` _asbase_character_bp))
      (`/Engine/EditorBlueprintResources/StandardMacros.IsValid` _returnvalue_2
        (:`Is Valid`
          (`self.SetActorHiddenInGame` _asbase_character_bp false))))))

(event `Disable`
  (bind _asplayer_hudcontroller (cast `/Game/Blueprints/CharacterUtility/PlayerHUDController` (`ChildActorComponent.ChildActor` (`self.HUDController`))))
  (`/Game/Blueprints/CharacterUtility/PlayerHUDController.Disappear` _asplayer_hudcontroller)
  (bind _asbase_character_bp (cast `/Game/Blueprints/Characters/BaseCharacter_BP` (`self.K2_GetPawn`)))
  (`self.SetActorHiddenInGame` _asbase_character_bp true)
  (`|ExecutionSequence`
    (:`then_0`
      (bind _returnvalue (`InfomorphUE4Character.GetCurrentWeapon` _asbase_character_bp))
      (`/Engine/EditorBlueprintResources/StandardMacros.IsValid` _returnvalue
        (:`Is Valid`
          (`self.SetActorHiddenInGame` _returnvalue true))))
    (:`then_1`
      (bind _returnvalue_2 (`InfomorphUE4Character.GetCurrentShield` _asbase_character_bp))
      (`/Engine/EditorBlueprintResources/StandardMacros.IsValid` _returnvalue_2
        (:`Is Valid`
          (`self.SetActorHiddenInGame` true))))))

(event `Key|F1`
  (params (Key :type "Key Structure" :default "AnyKey"))
  ;[1 1 1] Debug
  (:`Pressed`
    (set `self.bGodMode` (not (`self.bGodMode`)))))

(event `Key|F2`
  (params (Key :type "Key Structure" :default "AnyKey"))
  ;[1 1 1] Debug
  (:`Pressed`
    (`KismetSystemLibrary.ExecuteConsoleCommand` "RestartLevel")))

(event `Key|F3`
  (params (Key :type "Key Structure" :default "AnyKey"))
  ;[1 1 1] Debug
  (:`Pressed`
    (`GameplayStatics.OpenLevel` "SplashScreenMap")))

(event `Key|F4`
  (params (Key :type "Key Structure" :default "AnyKey"))
  (bind _returnvalue (`GameplayStatics.GetPlayerPawn` 0))
  (bind _transformcomponent (`PlayerCameraManager.TransformComponent` (`GameplayStatics.GetPlayerCameraManager` 0)))
  ;[1 1 1] Debug
  (:`Pressed`
    (`self.K2_TeleportTo` _returnvalue (+ (* (`SceneComponent.GetForwardVector` _transformcomponent) 200.0) (`self.K2_GetActorLocation` _returnvalue)) (`SceneComponent.K2_GetComponentRotation` _transformcomponent))))

(fn `UserConstructionScript`)
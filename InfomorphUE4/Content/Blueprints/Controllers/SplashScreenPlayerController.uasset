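; Player controller for the splash screen, showing a blinking "press any key" widget with a fade-in and background music.
; Gamepad bottom face button, Enter or E triggers LoadScene, guarded by a flag so it runs only once.
; LoadScene reverses the fade, shows a spinning loading indicator and fades out the music, then opens DemoMap after a short delay.
; A level-streaming alternative is left unconnected.
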(event `self.ReceiveBeginPlay`
  (bind _returnvalue (`|CreateWidget` "/Game/CustomContent/Blueprints/GUI/MenuPressAnyKey.MenuPressAnyKey_C" self))
  (bind _output_get (set `self.UI` _returnvalue))
  (`UserWidget.AddToViewport` _output_get 0)
  (`UserWidget.PlayAnimation` _output_get (`/Game/CustomContent/Blueprints/GUI/MenuPressAnyKey.Blink` _output_get) 0.0 0 "Forward" 1.0)
  (`UserWidget.PlayAnimation` _output_get (`/Game/CustomContent/Blueprints/GUI/MenuPressAnyKey.Fade` _output_get) 0.0 1 "Forward" 1.0)
  (bind _returnvalue_2 (`GameplayStatics.SpawnSound2D` "/Game/Audio/Ambients/Cues/bensound-scifi_Cue.bensound-scifi_Cue"))
  (set `self.Music` _returnvalue_2))

(event `Key|Gamepad_FaceButton_Bottom`
  (params (Key :type "Key Structure" :default "AnyKey"))
  (:`Pressed`
    (`self.LoadScene` :!label _label)))

(event `Key|Enter`
  (params (Key :type "Key Structure" :default "AnyKey"))
  (:`Pressed`
    (goto _label)))

(event `Key|E`
  (params (Key :type "Key Structure" :default "AnyKey"))
  (:`Pressed`
    (goto _label)))

(event `LoadScene`
  (bind _ui (`self.UI`))
  (if (not (`self.bLoadingScene`))
    (set `self.bLoadingScene` true)
    (`|ExecutionSequence`
      (:`then_0`
        (`UserWidget.PlayAnimation` _ui (`/Game/CustomContent/Blueprints/GUI/MenuPressAnyKey.Fade` _ui) 0.0 1 "Reverse" 1.0)
        (`UserWidget.PlayAnimation` _ui (`/Game/CustomContent/Blueprints/GUI/MenuPressAnyKey.LoadingRotatorFadeIn` _ui) 0.0 1 "Forward" 1.0)
        (`UserWidget.PlayAnimation` _ui (`/Game/CustomContent/Blueprints/GUI/MenuPressAnyKey.LoadingRotatorRotate` _ui) 0.0 0 "Forward" 1.0)
        (`AudioComponent.FadeOut` (`self.Music`) 1.0 0.0))
      (:`then_1`
        (`KismetSystemLibrary.Delay` 1.0)
        (`GameplayStatics.OpenLevel` "DemoMap")))))

(fn `UserConstructionScript`)
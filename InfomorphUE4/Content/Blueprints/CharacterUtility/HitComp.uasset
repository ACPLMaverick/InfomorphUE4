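; Hit component for characters and InfomorphShields that plays impact effects when another owner's InfomorphWeapon overlaps them.
; It binds to character mesh or shield actor overlaps, then sphere-traces from weapon to owner for impact point and normal.
; Each hit can spawn particles, sound and a random stream-picked decal, attached to the nearest skeletal bone, else another mesh or root.
; It applies no damage, and only the shield path seeds the random stream.
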(event `self.ReceiveBeginPlay`
  (bind _returnvalue (`self.GetOwner`))
  (bind _asbase_character_bp (cast `/Game/Blueprints/Characters/BaseCharacter_BP` _returnvalue)
    (:`then`
      (add `PrimitiveComponent.OnComponentBeginOverlap` (`Character.Mesh` _asbase_character_bp) (delegate `Meh`)))
    (:`CastFailed`
      (bind _asinfomorph_shield (cast `InfomorphShield` _returnvalue))
      (add `Actor.OnActorBeginOverlap` _asinfomorph_shield (delegate `OnShieldBeginOverlap`))
      (`KismetMathLibrary.SeedRandomStream` (`self.RandomStream`)))))

(event `Meh`
  (params (OverlappedComponent :type "PrimitiveComponent Object Reference") (OtherActor :type "Actor Object Reference") (OtherComp :type "PrimitiveComponent Object Reference") (OtherBodyIndex :type Integer) (bFromSweep :type Boolean) (SweepResult :type "HitResult Structure (by ref)"))
  (bind _asinfomorph_weapon (cast `InfomorphWeapon` OtherActor))
  (if (!= (`self.GetOwner` (`SceneComponent.GetAttachParent` (`Actor.K2_GetRootComponent` _asinfomorph_weapon))) (`self.GetOwner`))
    (bind (_loc _normal) (`self.GetOverlapData` _asinfomorph_weapon))
    (`self.MakeHitAtLocation` _loc _normal)))

(event `EventDamage`
  (params (DamagedActor :type "Actor Object Reference") (Damage :type "Float (double-precision)") (DamageType :type "DamageType Object Reference") (InstigatedBy :type "Controller Object Reference") (DamageCauser :type "Actor Object Reference")))

(event `OnShieldBeginOverlap`
  (params (OverlappedActor :type "Actor Object Reference") (OtherActor :type "Actor Object Reference"))
  (bind _asinfomorph_weapon (cast `InfomorphWeapon` OtherActor))
  (if (!= (`self.GetOwner` (`SceneComponent.GetAttachParent` (`Actor.K2_GetRootComponent` OverlappedActor))) (`self.GetOwner` (`SceneComponent.GetAttachParent` (`Actor.K2_GetRootComponent` _asinfomorph_weapon))))
    (bind (_loc _normal) (`self.GetOverlapData` _asinfomorph_weapon))
    (`self.MakeHitAtLocation` _loc _normal)))

(fn `GetDecalMaterial`
  (returns (Mat :type "MaterialInstanceConstant Object Reference"))
  (return (`|GetArrayItem` (`self.DecalMaterials`) (`KismetMathLibrary.RandomIntegerInRangeFromStream` 0 (- (`KismetArrayLibrary.Array_Length` (`self.DecalMaterials`)) 1) (`self.RandomStream`)))))

(fn `GetOverlapData`
  (params (Other :type "InfomorphWeapon Object Reference"))
  (returns (Loc :type "Vector Structure") (Normal :type "Vector Structure"))
  (bind _outhit (`KismetSystemLibrary.SphereTraceSingleForObjects` :`Start` (`Actor.K2_GetActorLocation` Other) :`End` (`Actor.K2_GetActorLocation` (`self.GetOwner`)) :`Radius` 1.0 :`ObjectTypes` (`|MakeArray` "ObjectTypeQuery3" :!type "EObjectTypeQuery Enum") :`bTraceComplex` true :`bIgnoreSelf` false))
  (bind (_bblockinghit _binitialoverlap _time _location _impactpoint _normal _impactnormal) (`GameplayStatics.BreakHitResult` _outhit))
  (return _impactpoint _impactnormal))

(fn `GetOwnerDecalAttachComponent`
  (params (DecalLocation :type "Vector Structure"))
  (returns (Point :type "SceneComponent Object Reference") (PointName :type Name))
  (bind _returnvalue (`self.GetOwner`))
  (bind _returnvalue_2 (`Actor.GetComponentByClass` _returnvalue "/Script/Engine.MeshComponent"))
  (if (`KismetSystemLibrary.IsValid` _returnvalue_2)
    (bind _asskeletal_mesh_component (cast `SkeletalMeshComponent` _returnvalue_2)
      (:`then`
        (return _asskeletal_mesh_component (`.ReturnValue` (`SkinnedMeshComponent.FindClosestBone_K2` _asskeletal_mesh_component DecalLocation 0.0 false))))
      (:`CastFailed`
        (return _returnvalue_2 "None")))
    (else
      (return (`Actor.K2_GetRootComponent` _returnvalue) "None"))))

(fn `IsMaterialsValid`
  (returns (IsValid :type Boolean))
  (return (> (`KismetArrayLibrary.Array_Length` (`self.DecalMaterials`)) 0)))

(fn `MakeHitAtLocation`
  (params (Location :type "Vector Structure") (Normal :type "Vector Structure"))
  (bind _particles (`self.Particles`))
  (bind _sound (`self.Sound`))
  (`|ExecutionSequence`
    (:`then_0`
      (`/Engine/EditorBlueprintResources/StandardMacros.IsValid` _particles
        (:`Is Valid`
          (bind _returnvalue (`GameplayStatics.SpawnEmitterAtLocation` (`self.GetOwner`) _particles Location))
          (`self.Activate` _returnvalue true)
          (`SceneComponent.SetWorldScale3D` _returnvalue (`KismetMathLibrary.MakeVector` 1.6 1.6 1.6)))))
    (:`then_1`
      (bind _isvalid (`self.IsMaterialsValid`))
      (if _isvalid
        (bind _mat (`self.GetDecalMaterial`))
        (bind (_point _pointname) (`self.GetOwnerDecalAttachComponent` Location))
        (`GameplayStatics.SpawnDecalAttached` _mat (`self.DecalSize`) _point _pointname (+ Location (* Normal 2.0)) (struct) "KeepWorldPosition" (`self.DecalLife`))))
    (:`then_2`
      (`/Engine/EditorBlueprintResources/StandardMacros.IsValid` _sound
        (:`Is Valid`
          (`GameplayStatics.PlaySoundAtLocation` (`self.GetOwner`) _sound Location))))))
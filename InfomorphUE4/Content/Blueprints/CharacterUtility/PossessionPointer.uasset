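; PossessionPointer is a pointer actor that visually links its parent character to the possessable character targeted by that character's camera.
; Each tick it rotates toward the target and scales along X by distance, keeping the last known location if the target becomes invalid.
; It also polls the parent's camera target while an InfomorphPlayerController_BP controls it, fading two planes through a shared dynamic material and a reversible opacity timeline.
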(event `self.ReceiveBeginPlay`
  (bind _plane (`self.Plane`))
  (bind _returnvalue (`PrimitiveComponent.CreateDynamicMaterialInstance` _plane 0 null))
  (bind _output_get (set `self.Mat` _returnvalue))
  (`PrimitiveComponent.SetMaterial` _plane 0 _output_get)
  (`PrimitiveComponent.SetMaterial` (`self.Plane2`) 0 _output_get)
  (`MaterialInstanceDynamic.SetScalarParameterValue` _output_get "Opacity" 0.0)
  (`self.SetActorHiddenInGame` true))

(event `self.ReceiveTick`
  (params (DeltaSeconds :type "Float (single-precision)"))
  (bind _returnvalue (`self.K2_GetActorLocation`))
  (bind _char (`self.Char`))
  (bind _returnvalue_2 (`KismetSystemLibrary.IsValid` _char))
  (bind _returnvalue_3 (and (`self.bVisible`) (not (`self.bFadeOut`))))
  (`|ExecutionSequence`
    (:`then_0`
      (if (or _returnvalue_2 (`self.bVisible`))
        (if _returnvalue_2
          (bind _output_get (set `self.CharLocation` (`self.K2_GetActorLocation` _char))))
        (`self.K2_SetActorRotation` (`KismetMathLibrary.FindLookAtRotation` _returnvalue _output_get))
        (`self.SetActorScale3D` (`KismetMathLibrary.MakeVector` (* (`KismetMathLibrary.VSize` (- _returnvalue _output_get)) 0.01) (.y (`self.GetActorScale3D`)) (.z (`self.GetActorScale3D`))))))
    (:`then_1`
      (bind _asbase_character_bp (cast `/Game/Blueprints/Characters/BaseCharacter_BP` (`self.GetParentActor`))
        (:`then`
          (cast `/Game/Blueprints/Controllers/InfomorphPlayerController_BP` (`Pawn.GetController` _asbase_character_bp)
            (:`then`
              (bind _returnvalue_4 (`InfomorphUE4Character.GetCameraTarget` _asbase_character_bp))
              (if (!= _returnvalue_4 (`self.Char`))
                (bind _asbase_character_bp_2 (cast `/Game/Blueprints/Characters/BaseCharacter_BP` _returnvalue_4)
                  (:`then`
                    (if (`InfomorphUE4Character.GetIsPossessable` _asbase_character_bp_2)
                      (`self.EventSetTarget` _asbase_character_bp_2)
                      (if (not (`self.bVisible`))
                        (`self.EventAppear`)
                        (else
                          (if (not (`KismetSystemLibrary.IsValid` (`self.Char`))) :!label _label
                            (`self.EventDisappear`))))
                      (elif _returnvalue_3
                        (`self.EventSetTarget` _asbase_character_bp_2)
                        (`self.EventDisappear`))))
                  (:`CastFailed`
                    (`self.EventSetTarget` _asbase_character_bp_2)
                    (goto _label)))))
            (:`CastFailed`
              (if _returnvalue_3 :!label _label_2
                (`self.EventDisappear`)
                (`KismetSystemLibrary.PrintString` "Hello")))))
        (:`CastFailed`
          (goto _label_2))))))

(event `EventAppear`
  (set `self.bVisible` true)
  (set `self.bFadeOut` false)
  (`self.SetActorHiddenInGame` false)
  (bind (_direction _opacity) (`Timeline|Timeline_0` :!via `PlayFromStart` :!label _label_3)
    (:`Update`
      (`MaterialInstanceDynamic.SetScalarParameterValue` (`self.Mat`) "Opacity" _opacity))
    (:`Finished`
      (if (`|EnumEquality` _direction "Backward")
        (`self.SetActorHiddenInGame` true)
        (set `self.bVisible` false)))))

(event `EventDisappear`
  (set `self.bFadeOut` true)
  (goto _label_3 :!via `ReverseFromEnd`))

(event `EventSetTarget`
  (params (Ac :type "/Game/Blueprints/Characters/BaseCharacter_BP Object Reference"))
  (set `self.Char` Ac))

(event `EventClearTarget`
  (set `self.Char` null))

(fn `UserConstructionScript`)
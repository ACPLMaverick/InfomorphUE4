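; Player HUD actor, attached as a child actor of InfomorphPlayerController_BP, that drives the HUD widget and screen effects for the possessed character.
; Each tick it pushes stats to the widget, toggles the interact prompt and strengthens a consciousness post-process as consciousness drops.
; The camera target, else the current interactable, gets a fading custom-depth highlight, with enemy color shifting by lost consciousness.
; The special attack icon index is stubbed to 0.
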(event `self.ReceiveBeginPlay`
  (bind _asinfomorph_player_controller_bp (cast `/Game/Blueprints/Controllers/InfomorphPlayerController_BP` (`self.GetParentActor`)))
  (bind _returnvalue (`|CreateWidget` "/Game/CustomContent/Blueprints/GUI/HUD.HUD_C" _asinfomorph_player_controller_bp))
  (`UserWidget.AddToViewport` _returnvalue 0)
  (bind _output_get (set `self.WidgetHUD` _returnvalue))
  (set `UserWidget.bIsFocusable` false _output_get)
  (bind _returnvalue_2 (`KismetMaterialLibrary.CreateDynamicMaterialInstance` "/Game/CustomContent/Materials/PostProcessHighlight.PostProcessHighlight"))
  (bind _output_get_2 (set `self.HighlightMaterialInstance` _returnvalue_2))
  (`PostProcessComponent.AddOrUpdateBlendable` (`self.PostProcess`) _output_get_2 1.0)
  (bind _returnvalue_3 (`KismetMaterialLibrary.CreateDynamicMaterialInstance` "/Game/CustomContent/Materials/PostProcessConsciousness.PostProcessConsciousness"))
  (bind _output_get_3 (set `self.ConsciousnessMaterialInstance` _returnvalue_3))
  (`PostProcessComponent.AddOrUpdateBlendable` (`self.PostProcess`) _output_get_3 1.0))

(event `self.ReceiveTick`
  (params (DeltaSeconds :type "Float (single-precision)"))
  (bind _bioiactionappeared (`self.bIOIActionAppeared`))
  (bind _widgethud (`self.WidgetHUD`))
  (bind _ioi_action (`/Game/CustomContent/Blueprints/GUI/HUD.IOI_Action` (`self.WidgetHUD`)))
  (bind _asinfomorph_player_controller_bp (cast `/Game/Blueprints/Controllers/InfomorphPlayerController_BP` (`self.GetParentActor`)))
  (bind _asinfomorph_template_character_bp (cast `/Game/Blueprints/Characters/InfomorphTemplateCharacter_BP` (`Controller.K2_GetPawn` _asinfomorph_player_controller_bp)))
  (`|ExecutionSequence`
    (:`then_0`
      (`/Engine/EditorBlueprintResources/StandardMacros.IsValid` _widgethud
        (:`Is Valid`
          (bind _skillindex (`self.GetAttackIndexFromPossessedCharacter` _asinfomorph_template_character_bp))
          (bind _returnvalue (/ (`InfomorphUE4Character.GetCurrentConsciousness` _asinfomorph_template_character_bp) (`InfomorphUE4Character.GetMaxConsciousness` _asinfomorph_template_character_bp)))
          (`/Game/CustomContent/Blueprints/GUI/PlayerStats.UpdateStats` (`/Game/CustomContent/Blueprints/GUI/HUD.PlayerStats` _widgethud) _returnvalue (/ (`InfomorphUE4Character.GetCurrentEnergy` _asinfomorph_template_character_bp) (`InfomorphUE4Character.GetMaxEnergy` _asinfomorph_template_character_bp)) (- 1.0 (`InfomorphUE4Character.GetRatioRemainingToActivateSpecialAttack` _asinfomorph_template_character_bp)) (- 1.0 (`InfomorphPlayerController.GetCurrentSkillRemainingRatio` _asinfomorph_player_controller_bp)) (`InfomorphPlayerController.GetCurrentSkillIndex` _asinfomorph_player_controller_bp) _skillindex))))
    (:`then_1`
      (bind _returnvalue_2 (`InfomorphUE4Character.GetCameraTarget` _asinfomorph_template_character_bp))
      (bind _returnvalue_3 (`KismetSystemLibrary.IsValid` _returnvalue_2))
      (bind _returnvalue_4 (`InfomorphPlayerController.GetCurrentInteractable` _asinfomorph_player_controller_bp))
      (bind _returnvalue_5 (`KismetSystemLibrary.IsValid` _returnvalue_4))
      (if (or _returnvalue_3 _returnvalue_5)
        (if _returnvalue_3
          (`self.SetActorTargeted` _returnvalue_2)
          (else
            (`self.SetActorTargeted` _returnvalue_4)))
        (set `self.HighlightTimer` (`KismetMathLibrary.FClamp` (+ (`self.HighlightTimer`) (* (`self.HighlightFadeSpeed`) (`GameplayStatics.GetWorldDeltaSeconds`)))))
        (`self.SetHighlightParams`)
        (elif (> (`self.HighlightTimer`) 0.0)
          (set `self.HighlightTimer` (`KismetMathLibrary.FClamp` (- (`self.HighlightTimer`) (* (`self.HighlightFadeSpeed`) (`GameplayStatics.GetWorldDeltaSeconds`)))))
          (`self.SetHighlightParams`)
          (elif (`KismetSystemLibrary.IsValid` (`self.TargetedActor`))
            (`self.UnsetTargetedActor`)))))
    (:`then_2`
      (`MaterialInstanceDynamic.SetScalarParameterValue` (`self.ConsciousnessMaterialInstance`) "Power" (`KismetMathLibrary.Square` (- 1.0 _returnvalue))))
    (:`then_3`
      (if (and _returnvalue_5 (not _bioiactionappeared))
        (set `self.bIOIActionAppeared` true)
        (`/Game/CustomContent/Blueprints/GUI/IconOfInterest.EventAppear` _ioi_action)
        (elif (and (not _returnvalue_5) _bioiactionappeared)
          (set `self.bIOIActionAppeared` false)
          (`/Game/CustomContent/Blueprints/GUI/IconOfInterest.EventDisappear` _ioi_action))))))

(fn `GetActorMeshes`
  (params (Ac :type "Actor Object Reference"))
  (returns (Ms :type "Array of MeshComponent Object Reference"))
  (return (`self.K2_GetComponentsByClass` Ac "/Script/Engine.MeshComponent")))

(fn `GetAttackIndexFromPossessedCharacter`
  (params (Chr :type "/Game/Blueprints/Characters/InfomorphTemplateCharacter_BP Object Reference"))
  (returns (SkillIndex :type Integer))
  (return 0))

(fn `LerpOfColor`
  (returns (Lerp :type "Float (double-precision)"))
  (bind _asinfomorph_template_character_bp (cast `/Game/Blueprints/Characters/InfomorphTemplateCharacter_BP` (`self.TargetedActor`))
    (:`then`
      (return (`KismetMathLibrary.FClamp` (- 1.0 (/ (`InfomorphUE4Character.GetCurrentConsciousness` _asinfomorph_template_character_bp) (`InfomorphUE4Character.GetMaxConsciousness` _asinfomorph_template_character_bp))))))
    (:`CastFailed`
      (return 0.0))))

(fn `SetActorTargeted`
  (params (Ac :type "Actor Object Reference"))
  (bind _highlightcolorinteractable (`self.HighlightColorInteractable`))
  (if (!= Ac (`self.TargetedActor`))
    (`|ExecutionSequence`
      (:`then_0`
        (if (`KismetSystemLibrary.IsValid` (`self.TargetedActor`))
          (`self.UnsetTargetedActor`)))
      (:`then_1`
        (bind _ms (`self.GetActorMeshes` Ac))
        (for _array_element _ms
          (`PrimitiveComponent.SetRenderCustomDepth` _array_element true)))
      (:`then_2`
        (set `self.HighlightTimer` 0.0))
      (:`then_3`
        (cast `/Game/Blueprints/Characters/InfomorphTemplateCharacter_BP` Ac
          (:`then`
            (set `self.TargetedColor` (`self.HighlightColorEnemy`))
            (set `self.TargetedColorB` (`self.HighlightColorEnemyLowHP`)))
          (:`CastFailed`
            (set `self.TargetedColor` _highlightcolorinteractable)
            (set `self.TargetedColorB` _highlightcolorinteractable))))
      (:`then_4`
        (set `self.TargetedActor` Ac)))))

(fn `SetHighlightParams`
  (bind _highlightmaterialinstance (`self.HighlightMaterialInstance`))
  (`MaterialInstanceDynamic.SetScalarParameterValue` _highlightmaterialinstance "HighlightAmount" (`self.HighlightTimer`))
  (bind _lerp (`self.LerpOfColor`))
  (`MaterialInstanceDynamic.SetVectorParameterValue` _highlightmaterialinstance "HighlightColor" (`KismetMathLibrary.LinearColorLerp` (`self.TargetedColor`) (`self.TargetedColorB`) _lerp)))

(fn `UnsetTargetedActor`
  (bind _ms (`self.GetActorMeshes` (`self.TargetedActor`)))
  (for _array_element _ms
    (`PrimitiveComponent.SetRenderCustomDepth` _array_element false)
    (set `self.TargetedActor` null)))

(fn `UserConstructionScript`)
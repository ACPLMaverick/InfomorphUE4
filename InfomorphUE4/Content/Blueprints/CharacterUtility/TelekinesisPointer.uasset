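; Telekinesis pointer, a child actor of a character that visually links it to the telekinetic pawn while a skill is in use.
; Starts hidden; Tick shows it and stores the pawn when the player's camera target is a telekinetic pawn during skill use.
; It hides once that target is gone and the skill ends.
; While tracking, it rotates toward the pawn and stretches its X scale to the distance between them.
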(event `self.ReceiveBeginPlay`
  (`self.SetActorHiddenInGame` true))

(event `self.ReceiveTick`
  (params (DeltaSeconds :type "Float (single-precision)"))
  (bind _returnvalue (`self.K2_GetActorLocation`))
  (bind _returnvalue_2 (`self.K2_GetActorLocation` (`self.Pawn`)))
  (`|ExecutionSequence`
    (:`then_0`
      (bind _asbase_character_bp (cast `/Game/Blueprints/Characters/BaseCharacter_BP` (`self.GetParentActor`)))
      (bind _asinfomorph_player_controller_bp (cast `/Game/Blueprints/Controllers/InfomorphPlayerController_BP` (`Pawn.GetController` _asbase_character_bp))
        (:`then`
          (bind _asinfomorph_telekinetic_pawn (cast `InfomorphTelekineticPawn` (`InfomorphUE4Character.GetCameraTarget` _asbase_character_bp))
            (:`then`
              (bind _returnvalue_3 (`InfomorphPlayerController.IsUsingSkill` _asinfomorph_player_controller_bp))
              (if (and (not (`self.bVisible`)) _returnvalue_3)
                (set `self.bVisible` true)
                (`self.SetActorHiddenInGame` false)
                (set `self.Pawn` _asinfomorph_telekinetic_pawn)))
            (:`CastFailed`
              (if (and (`self.bVisible`) (not _returnvalue_3)) :!label _label
                (set `self.bVisible` false)
                (`self.SetActorHiddenInGame` true)
                (set `self.Pawn` null)))))
        (:`CastFailed`
          (goto _label))))
    (:`then_1`
      (`/Engine/EditorBlueprintResources/StandardMacros.IsValid` (`self.Pawn`)
        (:`Is Valid`
          (`self.SetActorScale3D` (`KismetMathLibrary.MakeVector` (* (`KismetMathLibrary.VSize` (- _returnvalue _returnvalue_2)) 0.01) (.y (`self.GetActorScale3D`)) (.z (`self.GetActorScale3D`))))
          (`self.K2_SetActorRotation` (`KismetMathLibrary.FindLookAtRotation` _returnvalue _returnvalue_2)))))))

(fn `UserConstructionScript`)
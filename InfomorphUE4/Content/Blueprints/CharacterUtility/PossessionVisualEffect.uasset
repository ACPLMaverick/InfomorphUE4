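; Visual effect actor for character possession, attached to the possessing or newly possessed character and driven by a Progress value on Tick.
; Buildup raises a camera-facing distortion plane and fades the character's Z mask, then particles lerp toward the target character.
; PossessionBecome plays the plane and mask in reverse.
; Success and failure trigger timed post-process blendables through dynamic materials, with failure stepping its fade channels.
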(event `self.ReceiveBeginPlay`
  (bind _distortionplane (`self.DistortionPlane`))
  (bind _returnvalue (`KismetMaterialLibrary.CreateDynamicMaterialInstance` "/Game/CustomContent/Materials/PostProcessPossessionSuccess.PostProcessPossessionSuccess"))
  (bind _output_get (set `self.PostProcessSuccessMaterialInstance` _returnvalue))
  (`PostProcessComponent.AddOrUpdateBlendable` (`self.PostProcess`) _output_get 0.0)
  (bind _returnvalue_2 (`KismetMaterialLibrary.CreateDynamicMaterialInstance` "/Game/CustomContent/Materials/PostProcessPossessionFailure.PostProcessPossessionFailure"))
  (bind _output_get_2 (set `self.PostProcessFailureMaterialInstance` _returnvalue_2))
  (`PostProcessComponent.AddOrUpdateBlendable` (`self.PostProcess`) _output_get_2 0.0)
  (`self.DisableAll`)
  (bind _returnvalue_3 (`PrimitiveComponent.CreateDynamicMaterialInstance` _distortionplane 0 (`PrimitiveComponent.GetMaterial` _distortionplane 0)))
  (set `self.DistortionPlaneMaterialInstance` _returnvalue_3)
  (set `self.BaseParticleLocation` (`KismetMathLibrary.MakeVector` (.x (`SceneComponent.RelativeLocation` (`self.PossessionParticles`))) (.y (`SceneComponent.RelativeLocation` (`self.PossessionParticles`))) (* (.z (`SceneComponent.RelativeLocation` (`self.PossessionParticles`))) 0.5)))
  (if (`self.bEnabledBecoming`)
    (`SceneComponent.SetVisibility` (`self.DistortionPlane`) true false)
    (`MaterialInstanceDynamic.SetScalarParameterValue` (`self.DistortionPlaneMaterialInstance`) "Progress" 1.0)))

(event `self.ReceiveTick`
  (params (DeltaSeconds :type "Float (single-precision)"))
  (bind _distortionplane (`self.DistortionPlane`))
  (bind _possessedcharacter (`self.PossessedCharacter`))
  (`|ExecutionSequence`
    (:`then_0`
      (if (`self.bEnabled`)
        (`|ExecutionSequence`
          (:`then_0`
            (if (`self.bAutoProgress`)
              (set `self.Progress` (+ (`self.Progress`) (* (`GameplayStatics.GetWorldDeltaSeconds`) (`self.ProgressAutoSpeed`))))))
          (:`then_1`
            (bind _newparam (`self.IsBuildup`))
            (if _newparam
              (bind _ret (`self.GetBuildupProgress`))
              (`MaterialInstanceDynamic.SetScalarParameterValue` (`self.DistortionPlaneMaterialInstance`) "Progress" _ret)
              (`MaterialInstanceDynamic.SetScalarParameterValue` (`self.CharacterMaterialInstance`) "PossessionZMask" (- 1.0 _ret))
              (bind _asinfomorph_swatcharacter_bp (cast `/Game/Blueprints/Characters/InfomorphSWATCharacter_BP` (`self.GetParentActor`)))
              (`self.PlacePlaneBeforeCamera` (`SceneComponent.K2_GetComponentLocation` (`InfomorphUE4Character.FollowCamera` _asinfomorph_swatcharacter_bp)))
              (else
                (if (`SceneComponent.bVisible` _distortionplane)
                  (`SceneComponent.SetVisibility` _distortionplane false false))
                (`self.GetPossessionProgress`)
                (`/Engine/EditorBlueprintResources/StandardMacros.IsValid` _possessedcharacter
                  (:`Is Valid`
                    (`self.PlaceParticlesBetweenCharacters` (`self.K2_GetActorLocation`) (`self.K2_GetActorLocation` _possessedcharacter))
                    (bind _bfinished (`self.IsProgressFinished`))
                    (if _bfinished
                      (`self.PossessionClear`)))
                  (:`Is Not Valid`
                    (`KismetSystemLibrary.PrintString` "This shouldn't happen.")))))))
        (elif (`self.bEnabledBecoming`)
          (bind _output_get (set `self.Progress` (- (`self.Progress`) (* (`GameplayStatics.GetWorldDeltaSeconds`) (`self.ProgressAutoSpeed`)))))
          (bind _returnvalue (`KismetMathLibrary.FClamp` _output_get))
          (`MaterialInstanceDynamic.SetScalarParameterValue` (`self.DistortionPlaneMaterialInstance`) "Progress" _returnvalue)
          (`MaterialInstanceDynamic.SetScalarParameterValue` (`self.CharacterMaterialInstance`) "PossessionZMask" (- 1.0 _returnvalue))
          (if (< _output_get 0.0)
            (set `self.Progress` 0.0)
            (`MaterialInstanceDynamic.SetScalarParameterValue` (`self.DistortionPlaneMaterialInstance`) "Progress" 0.0)
            (`MaterialInstanceDynamic.SetScalarParameterValue` (`self.CharacterMaterialInstance`) "PossessionZMask" 1.0)
            (`SceneComponent.SetVisibility` (`self.DistortionPlane`) false true)
            (set `self.bEnabledBecoming` false)))))
    (:`then_1`
      (`self.TickPossessionSuccess`)
      (`self.TickPossessionFailure`))))

(fn `DisableAll`
  (`SceneComponent.SetVisibility` (`self.DistortionPlane`) false false)
  (`ActorComponent.Deactivate` (`self.PossessionParticles`))
  (set `self.PossessedCharacter` null))

(fn `GetBuildupProgress`
  (returns (Ret :type "Float (double-precision)"))
  (return (`KismetMathLibrary.FClamp` (`self.Progress`))))

(fn `GetPossessionProgress`
  (returns (Progress :type "Float (double-precision)"))
  (return (`KismetMathLibrary.FClamp` (- (`self.Progress`) 1.0))))

(fn `IsBuildup`
  (returns (NewParam :type Boolean))
  (return (<= (`self.Progress`) 1.0)))

(fn `IsEnabled`
  (returns (bEnabled :type Boolean))
  (return (`self.bEnabled`)))

(fn `IsProgressFinished`
  (returns (bFinished :type Boolean))
  (return (> (`self.Progress`) 2.0)))

(fn `PlaceParticlesBetweenCharacters`
  (params (ThisPos :type "Vector Structure") (NextPos :type "Vector Structure"))
  (bind _progress (`self.GetPossessionProgress`))
  (`SceneComponent.K2_SetWorldLocation` (`self.PossessionParticles`) (+ (`KismetMathLibrary.VLerp` ThisPos NextPos _progress) (`self.BaseParticleLocation`)) false true))

(fn `PlacePlaneBeforeCamera`
  (params (CamLoc :type "Vector Structure"))
  (bind _distortionplane (`self.DistortionPlane`))
  (bind _returnvalue (`SceneComponent.K2_GetComponentLocation` _distortionplane))
  (bind _returnvalue_2 (`SceneComponent.K2_GetComponentLocation` (`self.DefaultSceneRoot`)))
  (bind _returnvalue_3 (+ _returnvalue_2 (* (`KismetMathLibrary.Normal` (`KismetMathLibrary.MakeVector` (.x (- CamLoc _returnvalue)) (.y (- CamLoc _returnvalue)))) (`KismetMathLibrary.VSize` (`KismetMathLibrary.MakeVector` (.x (- _returnvalue _returnvalue_2)) (.y (- _returnvalue _returnvalue_2)))))))
  (`SceneComponent.K2_SetWorldLocationAndRotation` _distortionplane _returnvalue_3 (`KismetMathLibrary.MakeRotator` (.roll (`KismetMathLibrary.FindLookAtRotation` _returnvalue_3 CamLoc)) (+ (.pitch (`KismetMathLibrary.FindLookAtRotation` _returnvalue_3 CamLoc)) 90.0) (.yaw (`KismetMathLibrary.FindLookAtRotation` _returnvalue_3 CamLoc))) false false))

(fn `PossessionBecome`
  (bind _postprocess (`self.PostProcess`))
  (bind _distortionplanematerialinstance (`self.DistortionPlaneMaterialInstance`))
  (bind _charactermaterialinstance (`self.CharacterMaterialInstance`))
  (set `self.bEnabledBecoming` true)
  (`SceneComponent.SetVisibility` (`self.DistortionPlane`) true false)
  (set `self.Progress` 1.0)
  (if (and (`KismetSystemLibrary.IsValid` _distortionplanematerialinstance) (`KismetSystemLibrary.IsValid` _charactermaterialinstance))
    (`MaterialInstanceDynamic.SetScalarParameterValue` _distortionplanematerialinstance "Progress" 1.0)
    (`MaterialInstanceDynamic.SetScalarParameterValue` _charactermaterialinstance "PossessionZMask" 0.0)
    (set `self.bTickPossessionSucceeded` true)
    (set `self.bTickPossessionFailed` false)
    (set `self.PossessionPostprocessTimer` 0.0)
    (`PostProcessComponent.AddOrUpdateBlendable` _postprocess (`self.PostProcessFailureMaterialInstance`) 0.0)
    (`PostProcessComponent.AddOrUpdateBlendable` _postprocess (`self.PostProcessSuccessMaterialInstance`) 1.0)))

(fn `PossessionBegin`
  (params (PossessedChar :type "/Game/Blueprints/Characters/InfomorphSWATCharacter_BP Object Reference"))
  (bind _possessionparticles (`self.PossessionParticles`))
  (`SceneComponent.SetVisibility` (`self.DistortionPlane`) true false)
  (set `self.bEnabled` true)
  (set `self.bEnabledBecoming` false)
  (set `self.Progress` 0.0)
  (set `self.PossessedCharacter` PossessedChar)
  (`ActorComponent.Activate` _possessionparticles true)
  (`SceneComponent.K2_SetRelativeLocation` _possessionparticles (`KismetMathLibrary.MakeVector` (.x (`self.BaseParticleLocation`)) (.y (`self.BaseParticleLocation`)) (* (.z (`self.BaseParticleLocation`)) 2.0)) false true))

(fn `PossessionClear`
  (set `self.Progress` 0.0)
  (set `self.bEnabled` false)
  (`self.DisableAll`)
  (`MaterialInstanceDynamic.SetScalarParameterValue` (`self.DistortionPlaneMaterialInstance`) "Progress" 0.0)
  (`MaterialInstanceDynamic.SetScalarParameterValue` (`self.CharacterMaterialInstance`) "PossessionZMask" 1.0))

(fn `PossessionFailure`
  (bind _postprocess (`self.PostProcess`))
  (set `self.bTickPossessionSucceeded` false)
  (set `self.bTickPossessionFailed` true)
  (set `self.PossessionPostprocessTimer` 0.0)
  (`PostProcessComponent.AddOrUpdateBlendable` _postprocess (`self.PostProcessFailureMaterialInstance`) 1.0)
  (`PostProcessComponent.AddOrUpdateBlendable` _postprocess (`self.PostProcessSuccessMaterialInstance`) 0.0))

(fn `RegisterCharacterMaterial`
  (params (Mat :type "MaterialInstanceDynamic Object Reference"))
  (`/Engine/EditorBlueprintResources/StandardMacros.IsValid` Mat
    (:`Is Valid`
      (set `self.CharacterMaterialInstance` Mat)
      (if (`self.bEnabledBecoming`)
        (`MaterialInstanceDynamic.SetScalarParameterValue` (`self.CharacterMaterialInstance`) "PossessionZMask" 0.0)))
    (:`Is Not Valid`
      (`KismetSystemLibrary.PrintString` "Material Instance is Null."))))

(fn `SetPossessionProgress`
  (params (Progress :type "Float (double-precision)"))
  (set `self.Progress` (`KismetMathLibrary.FClamp` Progress 0.0 2.0)))

(fn `TickPossessionFailure`
  (locals (TimePart :type "Float (double-precision)"))
  (bind _postprocessfailurematerialinstance (`self.PostProcessFailureMaterialInstance`))
  (bind _possessionpostprocessfailureduration (`self.PossessionPostprocessFailureDuration`))
  (if (`self.bTickPossessionFailed`)
    (set `self.PossessionPostprocessTimer` (+ (`self.PossessionPostprocessTimer`) (`GameplayStatics.GetWorldDeltaSeconds`)))
    (if (< (`self.PossessionPostprocessTimer`) (`self.PossessionPostprocessFailureDuration`))
      (set `local.TimePart` (/ (`self.PossessionPostprocessFailureDuration`) 8.0))
      (`MaterialInstanceDynamic.SetScalarParameterValue` _postprocessfailurematerialinstance "Power" (- 1.0 (/ (`KismetMathLibrary.FClamp` (* (`self.PossessionPostprocessTimer`) 4.0) 0.0 _possessionpostprocessfailureduration) _possessionpostprocessfailureduration)))
      (if (< (`self.PossessionPostprocessTimer`) (* (`local.TimePart`) 5.0))
        (`MaterialInstanceDynamic.SetVectorParameterValue` _postprocessfailurematerialinstance "ParamFade" (make `LinearColor` 1.0 1.0 1.0 0.0))
        (elif (< (`self.PossessionPostprocessTimer`) (* (`local.TimePart`) 6.0))
          (`MaterialInstanceDynamic.SetVectorParameterValue` _postprocessfailurematerialinstance "ParamFade" (make `LinearColor` 0.0 1.0 1.0 0.0))
          (elif (< (`self.PossessionPostprocessTimer`) (* (`local.TimePart`) 7.0))
            (`MaterialInstanceDynamic.SetVectorParameterValue` _postprocessfailurematerialinstance "ParamFade" (make `LinearColor` 0.0 0.0 1.0 0.0)))))
      (else
        (set `self.bTickPossessionFailed` false)
        (`PostProcessComponent.AddOrUpdateBlendable` (`self.PostProcess`) (`self.PostProcessFailureMaterialInstance`) 0.0)))))

(fn `TickPossessionSuccess`
  (if (`self.bTickPossessionSucceeded`)
    (set `self.PossessionPostprocessTimer` (+ (`self.PossessionPostprocessTimer`) (`GameplayStatics.GetWorldDeltaSeconds`)))
    (if (< (`self.PossessionPostprocessTimer`) (`self.PossessionPostprocessSuccessDuration`))
      (`MaterialInstanceDynamic.SetScalarParameterValue` (`self.PostProcessSuccessMaterialInstance`) "Progress" (/ (`self.PossessionPostprocessTimer`) (`self.PossessionPostprocessSuccessDuration`)))
      (else
        (set `self.bTickPossessionFailed` false)
        (`PostProcessComponent.AddOrUpdateBlendable` (`self.PostProcess`) (`self.PostProcessSuccessMaterialInstance`) 0.0)))))

(fn `UserConstructionScript`)
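; Enemy info display attached as a child of a BaseCharacter_BP, showing an EnemyInfo widget for that character.
; Each tick it appears only while the character is the player's camera target and not player-controlled, animating out with a delayed hide.
; It feeds the widget the consciousness ratio and toggles a possession-available indicator based on the player's location.
; The actor rotates every tick to face the player camera.
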(event `self.ReceiveBeginPlay`
  (`self.SetActorHiddenInGame` true))

(event `self.ReceiveTick`
  (params (DeltaSeconds :type "Float (single-precision)"))
  (bind _returnvalue (`GameplayStatics.GetPlayerController` 0))
  (bind _bhiddenhelper (`self.bHiddenHelper`))
  (bind _returnvalue_2 (not _bhiddenhelper))
  (bind _asbase_character_bp (cast `/Game/Blueprints/Characters/BaseCharacter_BP` (`self.GetParentActor`)))
  (bind _asenemy_info (cast `/Game/CustomContent/Blueprints/GUI/EnemyInfo` (`WidgetComponent.GetUserWidgetObject` (`self.Widget`))))
  (bind _asbase_character_bp_2 (cast `/Game/Blueprints/Characters/BaseCharacter_BP` (`Controller.K2_GetPawn` _returnvalue)))
  (`|ExecutionSequence`
    (:`then_0`
      (bind _asinfomorph_player_controller_bp (cast `/Game/Blueprints/Controllers/InfomorphPlayerController_BP` (`Pawn.GetController` _asbase_character_bp))
        (:`then`
          _)
        (:`CastFailed`
          _))
      (bind _returnvalue_3 (== (`InfomorphUE4Character.GetCameraTarget` _asbase_character_bp_2) (`self.GetParentActor`)))
      (bind _returnvalue_4 (`KismetSystemLibrary.IsValid` _asinfomorph_player_controller_bp))
      (if (or (and _returnvalue_2 (not _returnvalue_3)) (and _returnvalue_2 _returnvalue_4))
        (`/Game/CustomContent/Blueprints/GUI/EnemyInfo.WidgetDisappear` _asenemy_info)
        (set `self.bHiddenHelper` true)
        (`KismetSystemLibrary.Delay` 0.3)
        (if (`self.bHiddenHelper`)
          (`self.SetActorHiddenInGame` true))
        (elif (and _bhiddenhelper _returnvalue_3 (not _returnvalue_4))
          (`self.SetActorHiddenInGame` false)
          (`/Game/CustomContent/Blueprints/GUI/EnemyInfo.WidgetAppear` _asenemy_info)
          (set `self.bHiddenHelper` false))))
    (:`then_1`
      (`/Game/CustomContent/Blueprints/GUI/EnemyInfo.SetConscioussessPercentage` _asenemy_info (/ (`InfomorphUE4Character.GetCurrentConsciousness` _asbase_character_bp) (`InfomorphUE4Character.GetMaxConsciousness` _asbase_character_bp))))
    (:`then_2`
      (bind _returnvalue_5 (`InfomorphUE4Character.GetIsPossessable` _asbase_character_bp (`self.K2_GetActorLocation` _asbase_character_bp_2)))
      (if (and _returnvalue_5 (not (`self.bIsShowingPossessable`)))
        (set `self.bIsShowingPossessable` true)
        (`/Game/CustomContent/Blueprints/GUI/EnemyInfo.IndicatePossessionAvailable` _asenemy_info)
        (elif (and (not _returnvalue_5) (`self.bIsShowingPossessable`))
          (set `self.bIsShowingPossessable` false)
          (`/Game/CustomContent/Blueprints/GUI/EnemyInfo.ClearPossessionAvailable` _asenemy_info))))
    (:`then_3`
      (`self.K2_SetActorRotation` (`KismetMathLibrary.FindLookAtRotation` (`self.K2_GetActorLocation`) (`PlayerCameraManager.GetCameraLocation` (`PlayerController.PlayerCameraManager` _returnvalue)))))))

(fn `UserConstructionScript`)
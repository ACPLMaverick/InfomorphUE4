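; SWAT character Blueprint that drives a digitalization effect on the head material during death.
; On BeginPlay it creates a dynamic instance of the mesh's second material slot, if present, and stores it as the head material.
; While TickDeath is set, Tick copies DeathAccumulator into that material's "Digtalization" scalar parameter, with no validity check on the instance.
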(event `self.ReceiveBeginPlay`
  (bind _mesh (`self.Mesh`))
  (`parent.ReceiveBeginPlay`)
  (if (> (`PrimitiveComponent.GetNumMaterials` _mesh) 1)
    (bind _returnvalue (`PrimitiveComponent.CreateDynamicMaterialInstance` _mesh 1 (`PrimitiveComponent.GetMaterial` _mesh 1)))
    (set `self.HeadMatInstance` _returnvalue)))

(event `self.ReceiveTick`
  (params (DeltaSeconds :type "Float (single-precision)"))
  (`parent.ReceiveTick` DeltaSeconds)
  (if (`self.bTickDeath`)
    (`MaterialInstanceDynamic.SetScalarParameterValue` (`self.HeadMatInstance`) "Digtalization" (`self.DeathAccumulator`))))

(fn `UserConstructionScript`
  (`parent.UserConstructionScript`))
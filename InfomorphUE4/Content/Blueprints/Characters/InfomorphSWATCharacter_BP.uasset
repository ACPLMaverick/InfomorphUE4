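; SWAT character Blueprint that drives possession and death visual feedback.
; On BeginPlay it registers its material with a PossessionVisualEffect child actor, which possess, unpossess and possession-failure events switch between states.
; While player-controlled, Tick polls the possession skill to begin or clear the effect on a SWAT target and feed it progress summed from build-up and possession timer ratios.
; Tick also activates DeathEffect once consciousness runs out.
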(event `self.ReceiveBeginPlay`
  (bind _aspossession_visual_effect (cast `/Game/Blueprints/CharacterUtility/PossessionVisualEffect` (`ChildActorComponent.ChildActor` (`self.PossessionVisualEffect`))))
  (`/Game/Blueprints/CharacterUtility/PossessionVisualEffect.RegisterCharacterMaterial` _aspossession_visual_effect (`self.GetMaterialInstance`)))

(event `self.ReceiveTick`
  (params (DeltaSeconds :type "Float (single-precision)"))
  (`|ExecutionSequence`
    (:`then_0`
      (`/Engine/EditorBlueprintResources/StandardMacros.IsValid` (`self.GetMaterialInstance`)
        (:`Is Valid`
          (bind _asinfomorph_player_controller_bp (cast `/Game/Blueprints/Controllers/InfomorphPlayerController_BP` (`self.GetController`)))
          (bind _asinfomorph_skill_possession (cast `InfomorphSkillPossession` (`InfomorphPlayerController.GetCurrentSkill` _asinfomorph_player_controller_bp)))
          (bind _aspossession_visual_effect (cast `/Game/Blueprints/CharacterUtility/PossessionVisualEffect` (`ChildActorComponent.ChildActor` (`self.PossessionVisualEffect`))))
          (bind _benabled (`/Game/Blueprints/CharacterUtility/PossessionVisualEffect.IsEnabled` _aspossession_visual_effect))
          (bind _returnvalue (`InfomorphSkillPossession.IsBeingUsed` _asinfomorph_skill_possession))
          (if (and (not _benabled) _returnvalue)
            (bind _asinfomorph_template_character_bp (cast `/Game/Blueprints/Characters/InfomorphSWATCharacter_BP` (`InfomorphSkillPossession.GetPossessedCharacter` _asinfomorph_skill_possession)))
            (`/Game/Blueprints/CharacterUtility/PossessionVisualEffect.PossessionBegin` _aspossession_visual_effect _asinfomorph_template_character_bp)
            (elif (and _benabled (not _returnvalue))
              (`/Game/Blueprints/CharacterUtility/PossessionVisualEffect.PossessionClear` _aspossession_visual_effect)
              (elif (and _benabled _returnvalue)
                (bind _progress (`self.ComputePossessionProgress` _asinfomorph_skill_possession))
                (`/Game/Blueprints/CharacterUtility/PossessionVisualEffect.SetPossessionProgress` _aspossession_visual_effect _progress)))))
        (:`Is Not Valid`
          (`KismetSystemLibrary.PrintString` "Hello"))))
    (:`then_1`
      (if (and (<= (`self.GetCurrentConsciousness`) 0.0) (not (`ActorComponent.IsActive` (`self.DeathEffect`))))
        (`ActorComponent.Activate` (`self.DeathEffect`) true)))))

(event `self.ReceivePossessed`
  (params (NewController :type "Controller Object Reference"))
  (cast `/Game/Blueprints/Controllers/InfomorphPlayerController_BP` NewController)
  (bind _aspossession_visual_effect (cast `/Game/Blueprints/CharacterUtility/PossessionVisualEffect` (`ChildActorComponent.ChildActor` (`self.PossessionVisualEffect`))))
  (`/Game/Blueprints/CharacterUtility/PossessionVisualEffect.PossessionBecome` _aspossession_visual_effect))

(event `self.ReceiveUnpossessed`
  (params (OldController :type "Controller Object Reference"))
  (cast `/Game/Blueprints/Controllers/InfomorphPlayerController_BP` OldController)
  (bind _aspossession_visual_effect (cast `/Game/Blueprints/CharacterUtility/PossessionVisualEffect` (`ChildActorComponent.ChildActor` (`self.PossessionVisualEffect`))))
  (`/Game/Blueprints/CharacterUtility/PossessionVisualEffect.PossessionClear` _aspossession_visual_effect))

(event `self.EventPossessionFailed`
  (params (CharacterWantedToPossess :type "InfomorphUE4Character Object Reference"))
  (bind _aspossession_visual_effect (cast `/Game/Blueprints/CharacterUtility/PossessionVisualEffect` (`ChildActorComponent.ChildActor` (`self.PossessionVisualEffect`))))
  (`/Game/Blueprints/CharacterUtility/PossessionVisualEffect.PossessionFailure` _aspossession_visual_effect))

(fn `ComputePossessionProgress`
  (params (PossessionSkill :type "InfomorphSkillPossession Object Reference"))
  (returns (Progress :type "Float (double-precision)"))
  (return (+ (/ (`InfomorphSkillPossession.GetBuildUpTimer` PossessionSkill) (`InfomorphSkillPossession.GetBuildUpTime` PossessionSkill)) (/ (`InfomorphSkillPossession.GetPossessionTimer` PossessionSkill) (`InfomorphSkillPossession.GetPossessionTime` PossessionSkill)))))

(fn `UserConstructionScript`)
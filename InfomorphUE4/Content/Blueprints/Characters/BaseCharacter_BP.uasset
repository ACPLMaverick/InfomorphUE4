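; Base character Blueprint for Infomorph's possessable characters, handling possession, spawn and death feedback.
; Tick and possession events drive a PossessionVisualEffect child actor from the player's possession skill; player possession also raises consciousness to a minimum threshold.
; A "Digtalization" material scalar animates spawning via timeline and death via a Tick accumulator once consciousness runs out.
; Failure events forward to the possession effect or player HUD controller.
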(event `self.ReceiveBeginPlay`
  (bind _aspossession_visual_effect (cast `/Game/Blueprints/CharacterUtility/PossessionVisualEffect` (`ChildActorComponent.ChildActor` (`self.PossessionVisualEffect`))))
  (`/Game/Blueprints/CharacterUtility/PossessionVisualEffect.RegisterCharacterMaterial` _aspossession_visual_effect (`self.GetMaterialInstance`))
  (if (`self.bSpawnEffectAtBeginPlay`)
    (`self.EventSpawn`)))

(event `self.ReceiveTick`
  (params (DeltaSeconds :type "Float (single-precision)"))
  (`|ExecutionSequence`
    (:`then_0`
      (`/Engine/EditorBlueprintResources/StandardMacros.IsValid` (`self.GetMaterialInstance`)
        (:`Is Valid`
          (bind _asinfomorph_player_controller_bp (cast `/Game/Blueprints/Controllers/InfomorphPlayerController_BP` (`self.GetController`)))
          (bind _asinfomorph_skill_possession (cast `InfomorphSkillPossession` (`InfomorphPlayerController.GetCurrentSkill` _asinfomorph_player_controller_bp)))
          (bind _aspossession_visual_effect (cast `/Game/Blueprints/CharacterUtility/PossessionVisualEffect` (`ChildActorComponent.ChildActor` (`self.PossessionVisualEffect`))))
          (bind _benabled (`/Game/Blueprints/CharacterUtility/PossessionVisualEffect.IsEnabled` _aspossession_visual_effect))
          (bind _returnvalue (`InfomorphSkillPossession.IsBeingUsed` _asinfomorph_skill_possession))
          (if (and (not _benabled) _returnvalue)
            (bind _asbase_character_bp (cast `/Game/Blueprints/Characters/BaseCharacter_BP` (`InfomorphSkillPossession.GetPossessedCharacter` _asinfomorph_skill_possession)))
            (`/Game/Blueprints/CharacterUtility/PossessionVisualEffect.PossessionBegin` _aspossession_visual_effect _asbase_character_bp)
            (elif (and _benabled (not _returnvalue))
              (`/Game/Blueprints/CharacterUtility/PossessionVisualEffect.PossessionClear` _aspossession_visual_effect)
              (elif (and _benabled _returnvalue)
                (bind _progress (`self.ComputePossessionProgress` _asinfomorph_skill_possession))
                (`/Game/Blueprints/CharacterUtility/PossessionVisualEffect.SetPossessionProgress` _aspossession_visual_effect _progress)))))
        (:`Is Not Valid`
          (`KismetSystemLibrary.PrintString` "Hello"))))
    (:`then_1`
      (if (and (<= (`self.GetCurrentConsciousness`) 0.0) (not (`self.bTickDeath`)))
        (set `self.bTickDeath` true)
        (`ActorComponent.Activate` (`self.DeathEffect`) true)))
    (:`then_2`
      (if (`self.bTickDeath`)
        (bind _output_get (set `self.DeathAccumulator` (+ (`self.DeathAccumulator`) (/ (`GameplayStatics.GetWorldDeltaSeconds`) (`self.DeathEffectDuration`)))))
        (`MaterialInstanceDynamic.SetScalarParameterValue` (`self.GetMaterialInstance`) "Digtalization" _output_get)))))

(event `self.ReceivePossessed`
  (params (NewController :type "Controller Object Reference"))
  (cast `/Game/Blueprints/Controllers/InfomorphPlayerController_BP` NewController)
  (bind _aspossession_visual_effect (cast `/Game/Blueprints/CharacterUtility/PossessionVisualEffect` (`ChildActorComponent.ChildActor` (`self.PossessionVisualEffect`))))
  (`self.RegenerateConscioussnessAtPossession`)
  (`/Game/Blueprints/CharacterUtility/PossessionVisualEffect.PossessionBecome` _aspossession_visual_effect))

(event `self.ReceiveUnpossessed`
  (params (OldController :type "Controller Object Reference"))
  (cast `/Game/Blueprints/Controllers/InfomorphPlayerController_BP` OldController)
  (bind _aspossession_visual_effect (cast `/Game/Blueprints/CharacterUtility/PossessionVisualEffect` (`ChildActorComponent.ChildActor` (`self.PossessionVisualEffect`))))
  (`/Game/Blueprints/CharacterUtility/PossessionVisualEffect.PossessionClear` _aspossession_visual_effect))

(event `self.EventPossessionFailed`
  (params (CharacterWantedToPossess :type "InfomorphUE4Character Object Reference"))
  (bind _aspossession_visual_effect (cast `/Game/Blueprints/CharacterUtility/PossessionVisualEffect` (`ChildActorComponent.ChildActor` (`self.PossessionVisualEffect`))))
  (`/Game/Blueprints/CharacterUtility/PossessionVisualEffect.PossessionFailure` _aspossession_visual_effect))

(event `self.EventNotEnoughEnergy`
  (bind _asinfomorph_player_controller_bp (cast `/Game/Blueprints/Controllers/InfomorphPlayerController_BP` (`self.GetController`)))
  (bind _asplayer_hudcontroller (cast `/Game/Blueprints/CharacterUtility/PlayerHUDController` (`ChildActorComponent.ChildActor` (`/Game/Blueprints/Controllers/InfomorphPlayerController_BP.HUDController` _asinfomorph_player_controller_bp))))
  (`/Game/Blueprints/CharacterUtility/PlayerHUDController.IndicateFailureEnergy` _asplayer_hudcontroller))

(event `self.EventCooldownNotFinishedSkill`
  (bind _asinfomorph_player_controller_bp (cast `/Game/Blueprints/Controllers/InfomorphPlayerController_BP` (`self.GetController`)))
  (bind _asplayer_hudcontroller (cast `/Game/Blueprints/CharacterUtility/PlayerHUDController` (`ChildActorComponent.ChildActor` (`/Game/Blueprints/Controllers/InfomorphPlayerController_BP.HUDController` _asinfomorph_player_controller_bp))))
  (`/Game/Blueprints/CharacterUtility/PlayerHUDController.IndicateFailureCooldownSkill` _asplayer_hudcontroller))

(event `self.EventCooldownNotFinishedSpecial`
  (bind _asinfomorph_player_controller_bp (cast `/Game/Blueprints/Controllers/InfomorphPlayerController_BP` (`self.GetController`)))
  (bind _asplayer_hudcontroller (cast `/Game/Blueprints/CharacterUtility/PlayerHUDController` (`ChildActorComponent.ChildActor` (`/Game/Blueprints/Controllers/InfomorphPlayerController_BP.HUDController` _asinfomorph_player_controller_bp))))
  (`/Game/Blueprints/CharacterUtility/PlayerHUDController.IndicateFailureCooldownSpecial` _asplayer_hudcontroller))

(event `EventSpawn`
  (if (`KismetSystemLibrary.IsValid` (`self.GetMaterialInstance`))
    (`GameplayStatics.PlaySoundAtLocation` (`self.SpawnSound`) (`self.K2_GetActorLocation`))
    (bind (_direction _newtrack_0) (`Timeline|SpawnTimeline` :!via `PlayFromStart`)
      (:`Update`
        (`MaterialInstanceDynamic.SetScalarParameterValue` (`self.GetMaterialInstance`) "Digtalization" _newtrack_0)))
    (else
      (set `self.bSpawnEffectAtBeginPlay` true))))

(fn `ComputePossessionProgress`
  (params (PossessionSkill :type "InfomorphSkillPossession Object Reference"))
  (returns (Progress :type "Float (double-precision)"))
  (return (+ (/ (`InfomorphSkillPossession.GetBuildUpTimer` PossessionSkill) (`InfomorphSkillPossession.GetBuildUpTime` PossessionSkill)) (/ (`InfomorphSkillPossession.GetPossessionTimer` PossessionSkill) (`InfomorphSkillPossession.GetPossessionTime` PossessionSkill)))))

(fn `RegenerateConscioussnessAtPossession`
  (bind (_baseconsciousness _baseenergy _energyrecoverypersecond _energyrestorecooldown _consciousnessarmorwhenpossessed _consciousnesspercentpossessable) (break `CharacterStats` (`self.CharacterStats`)))
  (if (< (`self.GetCurrentConsciousnessPercent`) _consciousnesspercentpossessable)
    (`self.SetCurrentConsciousness` (* (`self.GetMaxConsciousness`) _consciousnesspercentpossessable))))

(fn `UserConstructionScript`)
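; EnemySpawner is an area-triggered spawner that keeps a target count of AI enemies inside its spawn area while the player is present.
; Overlap events track whether a player-controlled BaseCharacter is in the actor's bounds.
; On Tick, if the area is under the desired count and the player's pawn isn't the spawned class, a delay timer accumulates.
; When it elapses, it spawns the pawn with its behavior tree and calls EventSpawn.
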(event `self.ReceiveActorBeginOverlap`
  (params (OtherActor :type "Actor Object Reference"))
  (bind _asbase_character_bp (cast `/Game/Blueprints/Characters/BaseCharacter_BP` OtherActor))
  (cast `/Game/Blueprints/Controllers/InfomorphPlayerController_BP` (`Pawn.GetController` _asbase_character_bp))
  (set `self.bIsPlayerInArea` true))

(event `self.ReceiveActorEndOverlap`
  (params (OtherActor :type "Actor Object Reference"))
  (bind _asbase_character_bp (cast `/Game/Blueprints/Characters/BaseCharacter_BP` OtherActor))
  (cast `/Game/Blueprints/Controllers/InfomorphPlayerController_BP` (`Pawn.GetController` _asbase_character_bp))
  (set `self.bIsPlayerInArea` false))

(event `self.ReceiveTick`
  (params (DeltaSeconds :type "Float (single-precision)"))
  (if (< (`KismetArrayLibrary.Array_Length` (`PrimitiveComponent.GetOverlappingActors` (`self.SpawnArea`) (`self.ClassToSpawn`))) (`self.DesiredEnemyCount`))
    (if (and (!= (`GameplayStatics.GetObjectClass` (`GameplayStatics.GetPlayerCharacter` 0)) (`self.ClassToSpawn`)) (`self.bIsPlayerInArea`))
      (if (>= (`self.SpawnTimer`) (`self.SpawnDelay`))
        (set `self.SpawnTimer` 0.0)
        (`self.Spawn`)
        (else
          (set `self.SpawnTimer` (+ (`GameplayStatics.GetWorldDeltaSeconds`) (`self.SpawnTimer`))))))))

(event `Spawn`
  (bind _returnvalue (`AIBlueprintHelperLibrary.SpawnAIFromClass` (`self.ClassToSpawn`) (`self.BehaviourTreeToSpawn`) (.location (`SceneComponent.K2_GetComponentToWorld` (`self.SpawnLocation`))) (.rotation (`SceneComponent.K2_GetComponentToWorld` (`self.SpawnLocation`)))))
  (bind _asbase_character_bp (cast `/Game/Blueprints/Characters/BaseCharacter_BP` _returnvalue))
  (`/Game/Blueprints/Characters/BaseCharacter_BP.EventSpawn` _asbase_character_bp))

(fn `UserConstructionScript`)
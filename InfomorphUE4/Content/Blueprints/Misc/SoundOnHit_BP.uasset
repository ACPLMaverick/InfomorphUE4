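; SoundOnHit_BP is a component that plays a sound when its owning actor's static mesh hits something.
; On BeginPlay it finds the owner's StaticMeshComponent and binds to its hit event.
; Each hit plays the assigned sound at the impact location, with a short real-time cooldown to prevent rapid repeats.
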(event `self.ReceiveBeginPlay`
  (bind _output_get (set `self.StaticMesh` (`Actor.GetComponentByClass` (`self.GetOwner`) "/Script/Engine.StaticMeshComponent")))
  (add `PrimitiveComponent.OnComponentHit` _output_get (delegate `OnMeshHit`)))

(event `OnMeshHit`
  (params (HitComponent :type "PrimitiveComponent Object Reference") (OtherActor :type "Actor Object Reference") (OtherComp :type "PrimitiveComponent Object Reference") (NormalImpulse :type "Vector Structure") (Hit :type "HitResult Structure (by ref)"))
  (if (> (- (`GameplayStatics.GetRealTimeSeconds`) (`self.LastHitTime`)) 0.25)
    (`GameplayStatics.PlaySoundAtLocation` (`self.SoundToPlay`) (`.Location` (`GameplayStatics.BreakHitResult` Hit)))
    (set `self.LastHitTime` (`GameplayStatics.GetRealTimeSeconds`))))
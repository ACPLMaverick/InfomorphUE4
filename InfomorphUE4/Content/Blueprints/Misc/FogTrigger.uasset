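; Trigger volume that changes the level's exponential height fog when the player enters it.
; A box overlap by a capsule on a character driven by the player controller captures the current fog density and height falloff.
; Tick then interpolates both toward the desired values at a set speed, snapping and stopping once both are within a small tolerance.
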(event `self.ReceiveBeginPlay`
  (add `PrimitiveComponent.OnComponentBeginOverlap` (`self.Box`) (delegate `CustomEvent_0`)))

(event `self.ReceiveTick`
  (params (DeltaSeconds :type "Float (single-precision)"))
  (bind _changespeed (`self.ChangeSpeed`))
  (if (`self.bLerpToValues`)
    (bind _asexponential_height_fog_component (cast `ExponentialHeightFogComponent` (`self.K2_GetRootComponent` (`self.LevelFog`))))
    (bind _output_get (set `self.CurrentDensity` (`KismetMathLibrary.FInterpTo` (`self.CurrentDensity`) (`self.DesiredDensity`) DeltaSeconds _changespeed)))
    (bind _output_get_2 (set `self.CurrentHeightFalloff` (`KismetMathLibrary.FInterpTo` (`self.CurrentHeightFalloff`) (`self.DesiredHeightFalloff`) DeltaSeconds _changespeed)))
    (`ExponentialHeightFogComponent.SetFogDensity` _asexponential_height_fog_component _output_get)
    (`ExponentialHeightFogComponent.SetFogHeightFalloff` _asexponential_height_fog_component _output_get_2)
    (bind _isfinished (`self.IsFinished`))
    (if _isfinished
      (set `self.bLerpToValues` false)
      (`ExponentialHeightFogComponent.SetFogDensity` _asexponential_height_fog_component (`self.DesiredDensity`))
      (`ExponentialHeightFogComponent.SetFogHeightFalloff` _asexponential_height_fog_component (`self.DesiredHeightFalloff`)))))

(event `CustomEvent_0`
  (params (OverlappedComponent :type "PrimitiveComponent Object Reference") (OtherActor :type "Actor Object Reference") (OtherComp :type "PrimitiveComponent Object Reference") (OtherBodyIndex :type Integer) (bFromSweep :type Boolean) (SweepResult :type "HitResult Structure (by ref)"))
  (cast `CapsuleComponent` OtherComp)
  (bind _isplayer (`self.IsPlayer` OtherActor))
  (bind _output_get (set `self.bLerpToValues` _isplayer))
  (if _output_get
    (bind _asexponential_height_fog_component (cast `ExponentialHeightFogComponent` (`self.K2_GetRootComponent` (`self.LevelFog`))))
    (set `self.CurrentDensity` (`ExponentialHeightFogComponent.FogDensity` _asexponential_height_fog_component))
    (set `self.CurrentHeightFalloff` (`ExponentialHeightFogComponent.FogHeightFalloff` _asexponential_height_fog_component))))

(fn `IsFinished`
  (returns (IsFinished :type Boolean))
  (return (and (< (`KismetMathLibrary.Abs` (- (`self.CurrentDensity`) (`self.DesiredDensity`))) 0.01) (< (`KismetMathLibrary.Abs` (- (`self.CurrentHeightFalloff`) (`self.DesiredHeightFalloff`))) 0.01))))

(fn `IsPlayer`
  (params (Ac :type "Actor Object Reference"))
  (returns (IsPlayer :type Boolean))
  (bind _asbase_character_bp (cast `/Game/Blueprints/Characters/BaseCharacter_BP` Ac)
    (:`then`
      (cast `/Game/Blueprints/Controllers/InfomorphPlayerController_BP` (`Pawn.GetController` _asbase_character_bp)
        (:`then`
          (return true))
        (:`CastFailed`
          _)))
    (:`CastFailed`
      _))
  (return false))

(fn `UserConstructionScript`)
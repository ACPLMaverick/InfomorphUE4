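; Trigger actor that shows an external message on the player's HUD when a player-controlled character overlaps it.
; It passes the message to the HUD controller child actor, along with the speech duration, and plays the optional speech as 2D sound.
; A PlayerIn flag blocks repeats until the player leaves, and the actor can optionally destroy itself after triggering.
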(event `self.ReceiveActorBeginOverlap`
  (params (OtherActor :type "Actor Object Reference"))
  (bind _message (`self.Message`))
  (bind _speech (`self.Speech`))
  (bind _asbase_character_bp (cast `/Game/Blueprints/Characters/BaseCharacter_BP` OtherActor))
  (bind _asinfomorph_player_controller_bp (cast `/Game/Blueprints/Controllers/InfomorphPlayerController_BP` (`Pawn.GetController` _asbase_character_bp)))
  (if (not (`self.bPlayerIn`))
    (`|ExecutionSequence`
      (:`then_0`
        (bind _asplayer_hudcontroller (cast `/Game/Blueprints/CharacterUtility/PlayerHUDController` (`ChildActorComponent.ChildActor` (`/Game/Blueprints/Controllers/InfomorphPlayerController_BP.HUDController` _asinfomorph_player_controller_bp))))
        (`/Engine/EditorBlueprintResources/StandardMacros.IsValid` _speech
          (:`Is Valid`
            (`/Game/Blueprints/CharacterUtility/PlayerHUDController.AddExternalMessage` _asplayer_hudcontroller _message (`SoundBase.Duration` _speech))
            (`GameplayStatics.PlaySound2D` _asinfomorph_player_controller_bp _speech))
          (:`Is Not Valid`
            (`/Game/Blueprints/CharacterUtility/PlayerHUDController.AddExternalMessage` _asplayer_hudcontroller _message 0.0))))
      (:`then_1`
        (if (`self.bDestroyAfterTriggered`)
          (`self.K2_DestroyActor`)))
      (:`then_2`
        (set `self.bPlayerIn` true)))))

(event `self.ReceiveActorEndOverlap`
  (params (OtherActor :type "Actor Object Reference"))
  (bind _asbase_character_bp (cast `/Game/Blueprints/Characters/BaseCharacter_BP` OtherActor))
  (cast `/Game/Blueprints/Controllers/InfomorphPlayerController_BP` (`Pawn.GetController` _asbase_character_bp))
  (set `self.bPlayerIn` false))

(fn `UserConstructionScript`)
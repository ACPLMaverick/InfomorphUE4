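; Trigger volume actor that ends the current play session with a "To Be Continued" screen.
; When the capsule of a player-controlled BaseCharacter_BP overlaps the box, it fires once, shows the ToBeContinued widget with its Appear animation, and disables player input.
; After a short delay it opens the splash screen map.
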(event `self.ReceiveBeginPlay`
  (add `PrimitiveComponent.OnComponentBeginOverlap` (`self.Box`) (delegate `CustomEvent_0`)))

(event `CustomEvent_0`
  (params (OverlappedComponent :type "PrimitiveComponent Object Reference") (OtherActor :type "Actor Object Reference") (OtherComp :type "PrimitiveComponent Object Reference") (OtherBodyIndex :type Integer) (bFromSweep :type Boolean) (SweepResult :type "HitResult Structure (by ref)"))
  (cast `CapsuleComponent` OtherComp)
  (if (not (`self.bActivated`))
    (bind _asbase_character_bp (cast `/Game/Blueprints/Characters/BaseCharacter_BP` OtherActor))
    (cast `/Game/Blueprints/Controllers/InfomorphPlayerController_BP` (`Pawn.GetController` _asbase_character_bp))
    (set `self.bActivated` true)
    (bind _returnvalue (`|CreateWidget` "/Game/CustomContent/Blueprints/GUI/ToBeContinued.ToBeContinued_C"))
    (`UserWidget.AddToViewport` _returnvalue 500)
    (`UserWidget.PlayAnimation` _returnvalue (`/Game/CustomContent/Blueprints/GUI/ToBeContinued.Appear` _returnvalue) 0.0 1 "Forward" 1.0)
    (`self.DisableInput` (`GameplayStatics.GetPlayerController` 0) null)
    (`KismetSystemLibrary.Delay` 6.0)
    (`GameplayStatics.OpenLevel` "SplashScreenMap")))

(fn `UserConstructionScript`)
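; Energy barrier that opens or blocks depending on the class of the characters inside its overlap zone.
; A lone exact match of PassableCharacterClass opens it, other arrivals block it, and removals reopen it when only matches remain or reset it when empty.
; States toggle plane collision and play sounds.
; Tick eases dynamic material parameters and both light colors toward the state, and drops dead characters from the zone.
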(event `self.ReceiveBeginPlay`
  (bind _returnvalue (`PrimitiveComponent.CreateDynamicMaterialInstance` (`self.Plane`) 0 null))
  (set `self.MatInstance` _returnvalue))

(event `self.ReceiveTick`
  (params (DeltaSeconds :type "Float (single-precision)"))
  (bind _lerpspeed (`self.LerpSpeed`))
  (bind _matinstance (`self.MatInstance`))
  (bind _actorsinzone (`self.ActorsInZone`))
  (`|ExecutionSequence`
    (:`then_0`
      (if (`self.bLerp`)
        (set `self.ValCurrentLerpMarkedDefault` (`KismetMathLibrary.FInterpTo` (`self.ValCurrentLerpMarkedDefault`) (`self.ValTargetLerpMarkedDefault`) DeltaSeconds _lerpspeed))
        (set `self.ValCurrentLerpBlockedPass` (`KismetMathLibrary.FInterpTo` (`self.ValCurrentLerpBlockedPass`) (`self.ValTargetLerpBlockedPass`) DeltaSeconds _lerpspeed))
        (if (and (< (`KismetMathLibrary.Abs` (- (`self.ValCurrentLerpMarkedDefault`) (`self.ValTargetLerpMarkedDefault`))) 0.01) (< (`KismetMathLibrary.Abs` (- (`self.ValCurrentLerpBlockedPass`) (`self.ValTargetLerpBlockedPass`))) 0.01))
          (set `self.ValCurrentLerpMarkedDefault` (`self.ValTargetLerpMarkedDefault`))
          (set `self.ValCurrentLerpBlockedPass` (`self.ValTargetLerpBlockedPass`))
          (set `self.bLerp` false))
        (`MaterialInstanceDynamic.SetScalarParameterValue` _matinstance "DefaultMarkedStateLerp" (`self.ValCurrentLerpMarkedDefault`))
        (`MaterialInstanceDynamic.SetScalarParameterValue` _matinstance "BlockedPassLerp" (`self.ValCurrentLerpBlockedPass`))
        (bind _color (`self.GetLightColor`))
        (`LightComponent.SetLightColor` (`self.Light_left`) _color true)
        (`LightComponent.SetLightColor` (`self.Light_right`) _color true)))
    (:`then_1`
      (for _array_element _actorsinzone
        (if (`InfomorphUE4Character.IsDead` _array_element)
          (`KismetArrayLibrary.Array_RemoveItem` _actorsinzone _array_element)
          (`self.ProcessActorRemoval` _array_element))))))

(event `self.ReceiveActorBeginOverlap`
  (params (OtherActor :type "Actor Object Reference"))
  (bind _actorsinzone (`self.ActorsInZone`))
  (bind _asbase_character_bp (cast `/Game/Blueprints/Characters/BaseCharacter_BP` OtherActor))
  (if (== (`KismetArrayLibrary.Array_Find` _actorsinzone _asbase_character_bp) -1)
    (`KismetArrayLibrary.Array_Add` _actorsinzone _asbase_character_bp)
    (`self.ProcessActorAddition` _asbase_character_bp)))

(event `self.ReceiveActorEndOverlap`
  (params (OtherActor :type "Actor Object Reference"))
  (bind _asbase_character_bp (cast `/Game/Blueprints/Characters/BaseCharacter_BP` OtherActor))
  (bind _returnvalue (`KismetArrayLibrary.Array_RemoveItem` (`self.ActorsInZone`) _asbase_character_bp))
  (if _returnvalue
    (`self.ProcessActorRemoval` _asbase_character_bp)))

(event `SetStateUnpassable`
  (bind _soundunpass (`self.SoundUnpass`))
  (if (`|EnumInequality` (`self.State`) "NewEnumerator1")
    (set `self.State` "NewEnumerator1")
    (set `self.ValTargetLerpMarkedDefault` 1.0)
    (set `self.ValTargetLerpBlockedPass` 0.0)
    (set `self.bLerp` true)
    (`PrimitiveComponent.SetCollisionEnabled` (`self.Plane`) "QueryAndPhysics")
    (if (`KismetSystemLibrary.IsValid` _soundunpass)
      (`GameplayStatics.PlaySoundAtLocation` self _soundunpass (`self.K2_GetActorLocation`)))))

(event `SetStatePassable`
  (bind _soundpass (`self.SoundPass`))
  (if (`|EnumInequality` (`self.State`) "NewEnumerator2")
    (set `self.State` "NewEnumerator2")
    (set `self.ValTargetLerpMarkedDefault` 1.0)
    (set `self.ValTargetLerpBlockedPass` 1.0)
    (set `self.bLerp` true)
    (`PrimitiveComponent.SetCollisionEnabled` (`self.Plane`) "NoCollision")
    (if (`KismetSystemLibrary.IsValid` _soundpass)
      (`GameplayStatics.PlaySoundAtLocation` self _soundpass (`self.K2_GetActorLocation`)))))

(event `SetStateDefault`
  (bind _sounddefault (`self.SoundDefault`))
  (if (`|EnumInequality` (`self.State`) "NewEnumerator0")
    (set `self.State` "NewEnumerator0")
    (set `self.ValTargetLerpMarkedDefault` 0.0)
    (set `self.ValTargetLerpBlockedPass` 0.0)
    (set `self.bLerp` true)
    (`PrimitiveComponent.SetCollisionEnabled` (`self.Plane`) "QueryAndPhysics")
    (if (`KismetSystemLibrary.IsValid` _sounddefault)
      (`GameplayStatics.PlaySoundAtLocation` self _sounddefault (`self.K2_GetActorLocation`)))))

(fn `GetLightColor`
  (returns (Color :type "LinearColor Structure"))
  (return (`KismetMathLibrary.LinearColorLerp` (`self.ColorLightDefault`) (`KismetMathLibrary.LinearColorLerp` (`self.ColorLightUnpassable`) (`self.ColorLightPassable`) (`self.ValCurrentLerpBlockedPass`)) (`self.ValCurrentLerpMarkedDefault`))))

(fn `IsPassable`
  (params (Char :type "/Game/Blueprints/Characters/BaseCharacter_BP Object Reference"))
  (returns (Passable :type Boolean))
  (return (== (`GameplayStatics.GetObjectClass` Char) (`self.PassableCharacterClass`))))

(fn `ProcessActorAddition`
  (params (Char :type "/Game/Blueprints/Characters/BaseCharacter_BP Object Reference"))
  (bind _passable (`self.IsPassable` Char))
  (if _passable
    (bind _result (`/Engine/EditorBlueprintResources/StandardMacros.IncrementInt` (`self.PassableCharactersInZone`))
      (:`  `
        (if (and (== _result 1) (== (`KismetArrayLibrary.Array_Length` (`self.ActorsInZone`)) 1))
          (`self.SetStatePassable`)
          (else
            (`self.SetStateUnpassable` :!label _label)))))
    (elif (`|EnumInequality` (`self.State`) "NewEnumerator1")
      (goto _label))))

(fn `ProcessActorRemoval`
  (params (Char :type "/Game/Blueprints/Characters/BaseCharacter_BP Object Reference"))
  (bind _passablecharactersinzone (`self.PassableCharactersInZone`))
  (bind _passable (`self.IsPassable` Char))
  (if _passable
    (bind _result (`/Engine/EditorBlueprintResources/StandardMacros.DecrementInt` _passablecharactersinzone)
      (:`  `
        (if (== _result 0)
          (if (and (== (`KismetArrayLibrary.Array_Length` (`self.ActorsInZone`)) _passablecharactersinzone) (!= _passablecharactersinzone 0)) :!label _label
            (`self.SetStatePassable`)
            (elif (== (`KismetArrayLibrary.Array_Length` (`self.ActorsInZone`)) 0)
              (`self.SetStateDefault`)
              (else
                (`self.SetStateUnpassable`))))
          (elif (and (== (`KismetArrayLibrary.Array_Length` (`self.ActorsInZone`)) _passablecharactersinzone) (!= _passablecharactersinzone 0))
            (`self.SetStatePassable`)))))
    (else
      (goto _label))))

(fn `UserConstructionScript`)
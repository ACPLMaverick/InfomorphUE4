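; A point light actor that pulses its intensity between a base level and a multiplied blink level.
; BeginPlay picks a random phase from a seeded stream, then either applies the exposed color, radius and shadow settings or adopts the light component's own intensity as the base.
; When Sinusoidal is set, Tick lerps intensity along a sine of game time, BlinkSpeed and phase; no other blink mode exists.
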(event `self.ReceiveBeginPlay`
  (bind _randoms (`self.Randoms`))
  (bind _pointlight (`self.PointLight`))
  (`KismetMathLibrary.SeedRandomStream` _randoms)
  (set `self.Phase` (`KismetMathLibrary.RandomFloatInRangeFromStream` (`self.BaseIntensity`) (`self.BlinkIntensity`) _randoms))
  (if (`self.bUseBaseVariables`)
    (set `self.BlinkIntensity` (* (`self.BaseIntensity`) (`self.BlinkIntensityMplier`)))
    (`LightComponent.SetLightColor` _pointlight (`self.BaseColor`) false)
    (`PointLightComponent.SetAttenuationRadius` _pointlight (`self.Attenuation`))
    (`LightComponentBase.SetCastShadows` _pointlight (`self.bCastShadows`))
    (else
      (bind _output_get (set `self.BaseIntensity` (`LightComponentBase.Intensity` _pointlight)))
      (set `self.BlinkIntensity` (* _output_get (`self.BlinkIntensityMplier`))))))

(event `self.ReceiveTick`
  (params (DeltaSeconds :type "Float (single-precision)"))
  (if (`self.bSinusoidal`)
    (`LightComponent.SetIntensity` (`self.PointLight`) (`KismetMathLibrary.Lerp` (`self.BaseIntensity`) (`self.BlinkIntensity`) (* (+ (`KismetMathLibrary.Sin` (+ (* (`KismetSystemLibrary.GetGameTimeInSeconds`) (`self.BlinkSpeed`)) (`self.Phase`))) 1.0) 0.5)))))

(fn `UserConstructionScript`)